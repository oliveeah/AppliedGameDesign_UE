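; TouchGameMode_BP is a game mode that links sign add and remove events to the on-screen UI and exposes level progress checks.
; On BeginPlay it creates UMG_UI, adds it to the viewport and binds two events that call the widget's Add and Remove.
; Three getters wrap checks for level completion, odd full and even full, which are not defined in this graph.
; An unconnected node setting the widget's iteration count never runs.
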(event Custom|CustomEvent
  (params (SignActor :type Actor%20Object%20Reference))
  (Default|Remove (Variables|Default|Getwidget)))

(event Custom|CustomEvent_0
  (params (SignActor :type Actor%20Object%20Reference))
  (Default|Add (Variables|Default|Getwidget)))

(event EventBeginPlay
  (bind _returnvalue (UserInterface|CreateWidget "/Game/blueprints/UMG_UI.UMG_UI_C" (Game|GetPlayerController 0)))
  (bind _output_get (Variables|Default|Setwidget _returnvalue))
  (UserInterface|Viewport|AddtoViewport _output_get 0)
  (EventDispatchers|BindEventtoOnSignAdded (delegate Custom|CustomEvent_0))
  (EventDispatchers|BindEventtoOnSignRemoved (delegate Custom|CustomEvent)))

(fn ConstructionScript)

(fn GetIsLevelComplete
  (bind _returnvalue (Class|TouchGameMode|CheckifLevelIsComplete self))
  (bind _output_get (Variables|Default|SetlocalIsLevelComplete _returnvalue))
  (return _output_get))

(fn GetIsOddFull
  (bind _returnvalue (Class|TouchGameMode|CheckifOddIsFull self))
  (bind _output_get (Variables|Default|SetlocalIsOddFull _returnvalue))
  (return _output_get))

(fn GetIsEvenFull
  (bind _returnvalue (Class|TouchGameMode|CheckifEvenIsFull self))
  (bind _output_get (Variables|Default|SetlocalIsEvenFull _returnvalue))
  (return _output_get))