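; Sheep variant of the grabbable chicken object Blueprint, which links the object's flying state and cry sounds to the sheep.
; On BeginPlay, without calling the parent's, it binds handlers to the flying-state and play-SFX events.
; The flying handler copies the flag into the ABP_sheepV2 anim instance, printing an error if the cast fails.
; The SFX handler passes the unique cry to the parent's play function.
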(event Custom|CustomEvent
  (params (bisFlying :type Boolean))
  (bind _output_get (Variables|Default|Setlocal_isFlying bisFlying))
  (bind _asabp_sheep_v2 (Utilities|Casting|CastToABP_sheepV2 (Components|SkeletalMesh|GetAnimInstance (Variables|Character|GetMesh)))
    (:then
      (Variables|/Game/blueprints/animationBlueprints/ABP_sheepV2.ABP_sheepV2_C|Setabp_isflying _asabp_sheep_v2 _output_get))
    (:CastFailed
      (Development|PrintString "cast failed"))))

(event EventPlaySFXCustomEvent
  (params (uniqueCry :type Sound%20Base%20Object%20Reference))
  (CallFunction|PlaySFXFn uniqueCry))

(event Collision|EventActorBeginOverlap
  (params (OtherActor :type Actor%20Object%20Reference))
  (|CallParentFunction OtherActor) ; This node is disabled and will not be called.\nDrag off pins to build functionality.
)

(event EventBeginPlay
  (EventDispatchers|AssignOnMyEvent (delegate Custom|CustomEvent))
  (EventDispatchers|BindEventtoPlaySFXEvent (delegate EventPlaySFXCustomEvent)))

(event EventTick
  (params (DeltaSeconds :type Float%20%28single-precision%29)))

(fn ConstructionScript
  (|CallParentFunction))

(fn PlaySFXFn
  (params (soundBase :type Sound%20Base%20Object%20Reference))
  (|CallParentFunction soundBase))